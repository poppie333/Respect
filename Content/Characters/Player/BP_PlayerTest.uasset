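; Test player Blueprint that handles the inventory screen and a debug inventory printout.
; BeginPlay creates the inventory widget; I pushes each Inventory entry into its slots, a refresh noted as misplaced here, then FlipFlops the widget on and off screen along with mouse cursor and look/move input blocking.
; G calls PrintInventory, and the BPKillerSummon event fires GomiDispatcher.
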(event EventBeginPlay
  ;[1 1 1] 開始時にインベントリウィジェット作成
  (bind _returnvalue (UserInterface|CreateWidget "/Game/Items/Test/WBP_Inventory.WBP_Inventory_C"))
  (Variables|Default|SetInventoryWidget _returnvalue))

(event EventBPKillerSummon
  (Default|CallGomiDispatcher))

(event Input|KeyboardEvents|I
  (params (Key :type Key%20Structure :default "None"))
  (bind _returnvalue (Game|GetPlayerController 0))
  (bind _inventorywidget (Variables|Default|GetInventoryWidget))
  ;[1 1 1] インベントリ更新とインベントリを開く(インベントリ更新はここでしないようにする)
  (:Pressed
    (for (_array_element _array_index) (Variables|Default|GetInventory)
      (Default|AddSingleItemData (Variables|Default|GetInventoryWidget) (Variables|/Script/RespectClock.ItemBase|GetItemData _array_element) _array_index)
      (Utilities|Array|SetArrayElem (Utilities|Array|MakeArray "") _array_index (Variables|/Script/RespectClock.ItemBase|GetItemData _array_element)))
    (Utilities|FlowControl|FlipFlop
      (:A
        (UserInterface|Viewport|AddtoViewport _inventorywidget 0)
        (Variables|/Script/Engine.PlayerController|SetbShowMouseCursor _returnvalue true)
        (Input|SetIgnoreLookInput _returnvalue true)
        (Input|SetIgnoreMoveInput _returnvalue true))
      (:B
        (Widget|RemovefromParent _inventorywidget)
        (Variables|/Script/Engine.PlayerController|SetbShowMouseCursor _returnvalue false)
        (Input|SetIgnoreLookInput _returnvalue false)
        (Input|SetIgnoreMoveInput _returnvalue false)))))

(event Input|KeyboardEvents|G
  (params (Key :type Key%20Structure :default "None"))
  ;[1 1 1] デバッグ用　インベントリ内容表示
  (:Pressed
    (Class|PlayerCharacter|PrintInventory)))

(fn ConstructionScript)